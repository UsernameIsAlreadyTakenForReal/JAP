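; Game state Blueprint for Agoraphobia that sets how many spheres the current map has.
; It switches on the current level name and assigns NumberOfSpheres for the Stairway, Outside Back, Outside Front, Market and Street maps.
; The same lookup runs in the construction script and is repeated every Tick.
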(event EventBeginPlay)

(event EventTick
  (params (DeltaSeconds :type Float%20%28single-precision%29))
  (bind _returnvalue (Game|GetCurrentLevelName true))
  (switch string _returnvalue
    (:Map_Stairway
      (Variables|Default|SetNumberOfSpheres 3))
    (:Map_Outside_Back
      (Variables|Default|SetNumberOfSpheres 3))
    (:Map_Outside_Front
      (Variables|Default|SetNumberOfSpheres 2))
    (:Map_Market
      (Variables|Default|SetNumberOfSpheres 2))
    (:Map_Street
      (Variables|Default|SetNumberOfSpheres 8))))

(fn ConstructionScript
  (bind _returnvalue (Game|GetCurrentLevelName true))
  (switch string _returnvalue
    (:Map_Stairway
      (Variables|Default|SetNumberOfSpheres 3))
    (:Map_Outside_Back
      (Variables|Default|SetNumberOfSpheres 3))
    (:Map_Outside_Front
      (Variables|Default|SetNumberOfSpheres 2))
    (:Map_Market
      (Variables|Default|SetNumberOfSpheres 2))
    (:Map_Street
      (Variables|Default|SetNumberOfSpheres 8))))